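; BP_Checkpoint is a checkpoint actor that saves player data when interacted with.
; Sphere overlap stores a BPI_Player actor and reveals a widget, while any end overlap hides the widget without clearing the stored actor.
; The Interract event fetches that actor's player data through an interface message, passes it to the Game Instance to save, and prints a confirmation.
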(event `/Game/ThirdPerson/Blueprints/BPI_Interractable.Interract`
  (bind _overlapped_actor (`self.Overlapped Actor`))
  (if (`KismetSystemLibrary.DoesImplementInterface` _overlapped_actor "/Game/ThirdPerson/Blueprints/BPI_Player.BPI_Player_C")
    (bind _savegamedata (message `/Game/ThirdPerson/Blueprints/BPI_Player.GetPlayerData` _overlapped_actor))
    (message `/Game/ThirdPerson/BPI_SaveGame.SavePlayer` (`GameplayStatics.GetGameInstance`) _savegamedata false)
    (`KismetSystemLibrary.PrintString` "Gane Saved !")))

(event `self.Sphere.OnComponentBeginOverlap`
  (params (OverlappedComponent :type "PrimitiveComponent Object Reference") (OtherActor :type "Actor Object Reference") (OtherComp :type "PrimitiveComponent Object Reference") (OtherBodyIndex :type Integer) (bFromSweep :type Boolean) (SweepResult :type "HitResult Structure (by ref)"))
  (if (`KismetSystemLibrary.DoesImplementInterface` OtherActor "/Game/ThirdPerson/Blueprints/BPI_Player.BPI_Player_C")
    (set `self.Overlapped Actor` OtherActor)
    (`SceneComponent.SetHiddenInGame` (`self.Widget`) false false)))

(event `self.Sphere.OnComponentEndOverlap`
  (params (OverlappedComponent :type "PrimitiveComponent Object Reference") (OtherActor :type "Actor Object Reference") (OtherComp :type "PrimitiveComponent Object Reference") (OtherBodyIndex :type Integer))
  (`SceneComponent.SetHiddenInGame` (`self.Widget`) true false))

(fn `UserConstructionScript`)